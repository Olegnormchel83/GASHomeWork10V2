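; BP_Guard is an AI guard character that tracks whether it has the player in target and carries a weapon it can shoot via GAS.
; On BeginPlay it binds to its AIC_Guard controller's detected and lost events and grants the GA_Shoot ability.
; Weapon events move the mesh between hand and spine sockets, holstering it when the player is lost.
; Getter functions expose the target state and muzzle socket location.
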(event Custom|WeaponRemove
  (Transformation|AttachComponentToComponent (Variables|Default|GetWeaponMesh) (Variables|Character|GetMesh) "SpineWeaponSocket" "SnapToTarget" "SnapToTarget" "SnapToTarget" true))

(event Custom|OnPlayerDetected_Event
  (Variables|Default|SetPlayerInTarget true))

(event Custom|OnPlayerLost_Event
  (Variables|Default|SetPlayerInTarget false)
  (CallFunction|WeaponRemove))

(event Custom|WeaponTaken
  (Transformation|AttachComponentToComponent (Variables|Default|GetWeaponMesh) (Variables|Character|GetMesh) "WeaponSocket" "SnapToTarget" "SnapToTarget" "SnapToTarget" true))

(event EventBeginPlay
  (Utilities|FlowControl|Sequence
    (:then_0
      (bind _asaic_guard (Utilities|Casting|CastToAIC_Guard (Pawn|GetController)))
      (EventDispatchers|BindEventtoOnPlayerDetected _asaic_guard (delegate Custom|OnPlayerDetected_Event))
      (EventDispatchers|BindEventtoOnPlayerLost _asaic_guard (delegate Custom|OnPlayerLost_Event)))
    (:then_1
      (GameplayAbilities|GiveAbility (Variables|Default|GetAbilitySystem) "/Game/HW_06/GAS/Abilities/Shoot/GA_Shoot.GA_Shoot_C" 0 -1))))

(fn ConstructionScript)

(fn IsPlayerinTarget
  (return (Variables|Default|GetPlayerInTarget)))

(fn GetMuzzleSocketLocation
  (return (Transformation|GetSocketLocation (Variables|Default|GetWeaponMesh) "MuzzleSocket")))