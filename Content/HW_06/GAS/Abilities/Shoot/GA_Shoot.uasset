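; Gameplay Ability that fires a hitscan shot from a BP_Guard avatar.
; Once committed, it line-traces from the muzzle socket along the actor's forward vector, with debug drawing, and applies fixed damage through ApplyDamage to any blocking hit.
; It then applies GE_Shoot to the owner and ends, or cancels if the commit fails.
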(event Ability|EventActivateAbility
  (bind _returnvalue (Ability|CommitAbility))
  (if _returnvalue
    (bind _asbp_guard (Utilities|Casting|CastToBP_Guard (Ability|GetAvatarActorfromActorInfo)))
    (bind _outhit (Collision|LineTraceByChannel (Default|GetMuzzleSocketLocation _asbp_guard) (+ (Default|GetMuzzleSocketLocation _asbp_guard) (* (Transformation|GetActorForwardVector _asbp_guard) 1e+03)) "TraceTypeQuery3" false 0 "ForDuration" true "(R=1.000000,G=0.000000,B=0.000000,A=1.000000)" "(R=0.000000,G=1.000000,B=0.000000,A=1.000000)" 2.0))
    (if (.bBlockingHit (Collision|BreakHitResult _outhit))
      (Game|Damage|ApplyDamage (Components|GetOwner (.HitComponent (Collision|BreakHitResult _outhit))) 25.0 0 _asbp_guard))
    (Ability|ApplyGameplayEffectToOwner "/Game/HW_06/GAS/Abilities/Shoot/GE_Shoot.GE_Shoot_C")
    (Ability|EndAbility)
    (else
      (Ability|CancelAbility))))